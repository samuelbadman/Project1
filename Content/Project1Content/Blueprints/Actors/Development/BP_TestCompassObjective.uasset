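; Development test actor that places an objective marker on the player's HUD compass bar.
; On BeginPlay it adds a tinted objective icon at its location through the GameHUD's compass bar widget and stores the returned icon.
; When Move is enabled, Tick moves the actor along world Y at MoveSpeed and updates the icon's world location to follow.
; A delayed icon removal is present but disconnected.
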(event EventBeginPlay
  (bind _asgame_hud (Utilities|Casting|CastToGameHUD (HUD|GetHUD (Game|GetPlayerController 0))))
  (bind _returnvalue (Class|CompassBarUserWidget|AddCompassIcon (Class|GameHUDScreen|GetCompassBarWidget (Class|GameHUD|GetGameHUDScreen _asgame_hud)) "/Game/Project1Content/Textures/UI/Compass/T_CompassIcon_Objective.T_CompassIcon_Objective" (Utilities|Struct|MakeSlateColor (Variables|Default|GetCompassIconTint)) (Transformation|GetActorLocation)))
  (bind _output_get (Variables|Default|SetCompassIcon _returnvalue)))

(event EventTick
  (params (DeltaSeconds :type Float%20%28single-precision%29))
  (bind _compassicon (Variables|Default|GetCompassIcon))
  (if (Variables|Default|GetbMove)
    ;[0.15 0.15 0.15 0.5] Update actor location
    (Transformation|AddActorWorldOffset (Math|Vector|MakeVector 0.0 (* DeltaSeconds (Variables|Default|GetMoveSpeed)) 0.0))
    ;[0.15 0.15 0.15 0.5] Update icon location
    (Utilities|IsValid _compassicon
      (:Is%20Valid
        (Class|CompassIconUserWidget|SetWorldLocation _compassicon (Transformation|GetActorLocation))))))

(fn ConstructionScript)