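; Development test interactable that exercises the gameplay-tag-driven dialogue system with a branching two-response conversation.
; Interacting disables the player controller's interact component and plays the Start branch on the Dialogue component.
; The response functions pop the HUD's game modal layer and play their matching branch.
; Branch completions are printed, and finishing either response branch re-enables player interaction.
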(event OnDialogueBranchComplete(Dialogue)
  (params (CompletedBranch :type Gameplay%20Tag%20Structure%20%28by%20ref%29))
  (Development|PrintString (Utilities|String|Append "Dialogue branch completed: " (Utilities|String|ToString(Name) (GameplayTags|GetTagName CompletedBranch))))
  (if (or (== CompletedBranch "(TagName=\"Dialogue.TestDialogueInteractable.Response1\")") (== CompletedBranch "(TagName=\"Dialogue.TestDialogueInteractable.Response2\")"))
    (CallFunction|SetPlayerInteractEnabled true)))

(event Custom|SetPlayerInteractEnabled
  (params (Enable :type Boolean))
  (bind _asgame_player_controller (Utilities|Casting|CastToGamePlayerController (Game|GetPlayerController 0)))
  (if Enable
    (Class|PlayerInteractComponent|EnableInteract (Variables|/Script/Project1.GamePlayerController|GetPlayerInteractComponent _asgame_player_controller))
    (else
      (Class|PlayerInteractComponent|DisableInteract (Variables|/Script/Project1.GamePlayerController|GetPlayerInteractComponent _asgame_player_controller)))))

(event EventBeginPlay
  (bind _asproject_1hudbase (Utilities|Casting|CastToProject1HUDBase (HUD|GetHUD (Game|GetPlayerController 0))))
  (Variables|Default|SetProject1HUD _asproject_1hudbase))

(event EventOnInteractedwith
  (params (Interactor :type Actor%20Object%20Reference))
  (CallFunction|SetPlayerInteractEnabled false)
  (Class|DialogueComponent|PlayBranch (Variables|Default|GetDialogue) (GameplayTags|MakeLiteralGameplayTag "(TagName=\"Dialogue.TestDialogueInteractable.Branches.Start\")")))

(fn ConstructionScript)

(fn OnResponse1
  (CallFunction|PopGameModalWidgetLayer)
  (Class|DialogueComponent|PlayBranch (Variables|Default|GetDialogue) (GameplayTags|MakeLiteralGameplayTag "(TagName=\"Dialogue.TestDialogueInteractable.Response1\")")))

(fn OnResponse2
  (CallFunction|PopGameModalWidgetLayer)
  (Class|DialogueComponent|PlayBranch (Variables|Default|GetDialogue) (GameplayTags|MakeLiteralGameplayTag "(TagName=\"Dialogue.TestDialogueInteractable.Response2\")")))

(fn PopGameModalWidgetLayer
  (Class|Project1HUDBase|PopContentfromPrimaryLayoutWidgetLayer (Variables|Default|GetProject1HUD) (GameplayTags|MakeLiteralGameplayTag "(TagName=\"UI.Layers.Game.Modal\")")))

(fn GetInteractableDescription
  (return (Variables|Default|GetInteractableDescription)))