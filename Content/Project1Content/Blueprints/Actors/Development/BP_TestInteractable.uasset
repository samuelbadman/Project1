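; Development test interactable that serves as an example pickup, advertising a single-press "Pickup" action labeled with its display name.
; Interacting hides the actor and disables its cube's collision.
; Hold-interact events print debug messages and demonstrate dynamic gamepad rumble, with intensity derived linearly from hold progress.
; Save and Load persist the picked-up state by unique name through the game instance's save manager, reapplying the pickup on load.
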(event Custom|Pickup
  (Variables|Default|SetbPickedUp true)
  (Rendering|SetActorHiddenInGame true)
  (Collision|SetCollisionEnabled (Variables|Default|GetCube) "NoCollision"))

(event Custom|OnHoldInteractStarted_1
  (params (Interactor :type Actor%20Object%20Reference))
  ;[0.15 0.15 0.15 0.5] Long press interact with dynamic force feedback rumble example
  (Development|PrintString "Long press interact started")
  (Game|Feedback|PlayDynamicForceFeedback (Game|GetPlayerController 0) (* (Variables|Default|GetMaxLongPressGamepadRumbleIntensity) (/ (stale Custom|OnHoldInteractTicked_1 PercentComplete) 1e+02)) -1.0 false true false true))

(event Custom|OnHoldInteractTicked_1
  (params (Interactor :type Actor%20Object%20Reference) (DeltaTime :type Float%20%28single-precision%29) (PercentComplete :type Float%20%28single-precision%29))
  ;[0.15 0.15 0.15 0.5] Long press interact with dynamic force feedback rumble example
  (Development|PrintString (Utilities|String|Append "Long press interact ticked: " (Utilities|String|ToString(Float) PercentComplete)))
  (Game|Feedback|PlayDynamicForceFeedback (Game|GetPlayerController 0) (* (Variables|Default|GetMaxLongPressGamepadRumbleIntensity) (/ PercentComplete 1e+02)) -1.0 false true false true) ; enters at Update
)

(event Custom|OnHoldInteractCanceled_1
  (params (Interactor :type Actor%20Object%20Reference) (PercentComplete :type Float%20%28single-precision%29))
  ;[0.15 0.15 0.15 0.5] Long press interact with dynamic force feedback rumble example
  (Development|PrintString (Utilities|String|Append "LP canceled: " (Utilities|String|ToString(Float) PercentComplete)))
  (Game|Feedback|PlayDynamicForceFeedback (Game|GetPlayerController 0) (* (Variables|Default|GetMaxLongPressGamepadRumbleIntensity) (/ (stale Custom|OnHoldInteractTicked_1 PercentComplete) 1e+02)) -1.0 false true false true) ; enters at Stop
)

(event Custom|OnHoldInteractCompleted_1
  (params (Interactor :type Actor%20Object%20Reference))
  ;[0.15 0.15 0.15 0.5] Long press interact with dynamic force feedback rumble example
  (Development|PrintString "LP completed")
  (Game|Feedback|PlayDynamicForceFeedback (Game|GetPlayerController 0) (* (Variables|Default|GetMaxLongPressGamepadRumbleIntensity) (/ (stale Custom|OnHoldInteractTicked_1 PercentComplete) 1e+02)) -1.0 false true false true) ; enters at Stop
)

(event EventSave
  ;[0.15 0.15 0.15 0.5] Example of saving picked up state
  (bind _asproject_1game_instance_base (Utilities|Casting|CastToProject1GameInstanceBase (Game|GetGameInstance)))
  (Utilities|Map|Add (Variables|/Script/Project1.Project1SaveGame|GetStaticPickupSaveData (Class|SaveManager|GetGameSaveGameObject (Class|Project1GameInstanceBase|GetSaveManager _asproject_1game_instance_base))) (Utilities|String|StringToName (Class|Project1ActorBase|GetUniqueName)) (Utilities|Struct|MakePickupSaveData (Variables|Default|GetbPickedUp))))

(event EventLoad
  ;[0.15 0.15 0.15 0.5] Example of loading picked up state
  (bind _asproject_1game_instance_base (Utilities|Casting|CastToProject1GameInstanceBase (Game|GetGameInstance)))
  (Utilities|IsValid (Class|SaveManager|GetGameSaveGameObject (Class|Project1GameInstanceBase|GetSaveManager _asproject_1game_instance_base))
    (:Is%20Valid
      (if (.ReturnValue (Utilities|Map|Find (Variables|/Script/Project1.Project1SaveGame|GetStaticPickupSaveData (Class|SaveManager|GetGameSaveGameObject (Class|Project1GameInstanceBase|GetSaveManager _asproject_1game_instance_base))) (Utilities|String|StringToName (Class|Project1ActorBase|GetUniqueName))))
        (bind _output_get (Variables|Default|SetbPickedUp (Utilities|Struct|BreakPickupSaveData (.Value (Utilities|Map|Find (Variables|/Script/Project1.Project1SaveGame|GetStaticPickupSaveData (Class|SaveManager|GetGameSaveGameObject (Class|Project1GameInstanceBase|GetSaveManager _asproject_1game_instance_base))) (Utilities|String|StringToName (Class|Project1ActorBase|GetUniqueName)))))))
        (if _output_get
          (CallFunction|Pickup))))))

(event EventBeginPlay
  (Variables|Default|SetInteractableDescription (Utilities|Struct|MakeInteractableDescription (Utilities|String|StringToName (Utilities|String|Append "Pickup " (Utilities|GetDisplayName self))) "SinglePress")))

(event EventOnInteractedwith
  (params (Interactor :type Actor%20Object%20Reference))
  (Development|PrintString (Utilities|String|Append (Utilities|GetDisplayName self) " interacted with"))
  (CallFunction|Pickup))

(fn ConstructionScript)

(fn GetInteractableDescription
  (return (Variables|Default|GetInteractableDescription)))