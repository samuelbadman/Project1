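; Test interactable actor that opens a modal choice dialog when the player interacts with it, prompting "Make choice".
; On interact it disables the player's interact component and pushes a dynamic three-option modal onto the HUD's modal widget layer via option delegates.
; Each option prints its selection, pops the layer and re-enables interaction.
; An unconnected confirm/cancel modal example is also included but never runs.
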(event Custom|Option2Selected
  ;[0.15 0.15 0.15 0.5] Confirm modal example
  (Development|PrintString "Cancel selected...")
  (CallFunction|PopModalWIdgetLayer)
  (CallFunction|SetPlayerInteractEnabled true))

(event Custom|Option1Selected
  ;[0.15 0.15 0.15 0.5] Confirm modal example
  (Development|PrintString "Confirm selected...")
  (CallFunction|PopModalWIdgetLayer)
  (CallFunction|SetPlayerInteractEnabled true))

(event Custom|DynamicOption3Selected
  ;[0.15 0.15 0.15 0.5] Dynamic modal example
  (Development|PrintString "Option 3 selected...")
  (CallFunction|PopModalWIdgetLayer)
  (CallFunction|SetPlayerInteractEnabled true))

(event Custom|DynamicOption1Selected
  ;[0.15 0.15 0.15 0.5] Dynamic modal example
  (Development|PrintString "Option 1 selected...")
  (CallFunction|PopModalWIdgetLayer)
  (CallFunction|SetPlayerInteractEnabled true))

(event Custom|PopModalWIdgetLayer
  (bind _asproject_1hudbase (Utilities|Casting|CastToProject1HUDBase (HUD|GetHUD (Game|GetPlayerController 0))))
  (Class|Project1HUDBase|PopContentfromPrimaryLayoutWidgetLayer _asproject_1hudbase (GameplayTags|MakeLiteralGameplayTag "(TagName=\"UI.Layers.Game.Modal\")")))

(event Custom|DynamicOption2Selected
  ;[0.15 0.15 0.15 0.5] Dynamic modal example
  (Development|PrintString "Option 2 selected...")
  (CallFunction|PopModalWIdgetLayer)
  (CallFunction|SetPlayerInteractEnabled true))

(event Custom|SetPlayerInteractEnabled
  (params (Enable :type Boolean))
  (bind _asgame_player_controller (Utilities|Casting|CastToGamePlayerController (Game|GetPlayerController 0)))
  (if Enable
    (Class|PlayerInteractComponent|EnableInteract (Variables|/Script/Project1.GamePlayerController|GetPlayerInteractComponent _asgame_player_controller))
    (else
      (Class|PlayerInteractComponent|DisableInteract (Variables|/Script/Project1.GamePlayerController|GetPlayerInteractComponent _asgame_player_controller)))))

(event EventOnInteractedwith
  (params (Interactor :type Actor%20Object%20Reference))
  (CallFunction|SetPlayerInteractEnabled false)
  (bind _asproject_1hudbase (Utilities|Casting|CastToProject1HUDBase (HUD|GetHUD (Game|GetPlayerController 0))))
  ;[0.15 0.15 0.15 0.5] Dynamic modal example
  (Class|Project1HUDBase|PushDynamicModaltoWidgetLayer _asproject_1hudbase (GameplayTags|MakeLiteralGameplayTag "(TagName=\"UI.Layers.Game.Modal\")") (Variables|Default|GetDynamicModalScreenWidgetClass) "Test dynamic modal prompt text" (Utilities|Array|MakeArray (Utilities|Struct|MakeDynamicModalOptionData "Option 1" (delegate Custom|DynamicOption1Selected)) (Utilities|Struct|MakeDynamicModalOptionData "Option 2" (delegate Custom|DynamicOption2Selected)) (Utilities|Struct|MakeDynamicModalOptionData "Option 3" (delegate Custom|DynamicOption3Selected))) true))

(fn ConstructionScript)

(fn GetInteractActionText
  (return "Make choice"))